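; BP_Trap is a one-shot trap actor in Le_Labyrinthe that springs when the first-person player overlaps it.
; On overlap with BP_FirstPersonCharacter, it prints a debug message and jumps upward by a fixed Z offset in a single unswept move.
; An IsActivated flag, cleared on BeginPlay and set after the move, keeps it from triggering again, and nothing lowers it afterward.
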(event `self.ReceiveBeginPlay`
  (set `self.isActivated` false))

(event `self.ReceiveActorBeginOverlap`
  (params (OtherActor :type "Actor Object Reference"))
  ;[1 1 1] If player, add 200Z position
  (if (not (`self.isActivated`))
    (cast `/Game/Le_Labyrinthe/Blueprints/BP_FirstPersonCharacter` OtherActor)
    (`KismetSystemLibrary.PrintString` "Activate Trap")
    (`self.K2_SetActorLocation` (+ (`self.K2_GetActorLocation`) (0.0 0.0 170.0)))
    (set `self.isActivated` true)))

(fn `UserConstructionScript`)