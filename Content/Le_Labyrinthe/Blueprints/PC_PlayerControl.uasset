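; Player controller for the labyrinth game, turning Enhanced Input into first-person movement, mouse look and interaction.
; On BeginPlay it adds the player and interact mapping contexts and caches the first-person character, which it moves along control-rotation axes.
; Interact fires a line trace along the view direction, with persistent debug drawing, then a cast chain triggers the hit torch, switch or secret passage.
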(event `self.ReceiveBeginPlay`
  (bind _returnvalue (subsystem `EnhancedInputLocalPlayerSubsystem`))
  (`/Engine/EditorBlueprintResources/StandardMacros.IsValid` _returnvalue
    (:`Is Valid`
      (`EnhancedInputSubsystemInterface.AddMappingContext` _returnvalue "/Game/Le_Labyrinthe/Mapping/IMC_MappingContextPlayer.IMC_MappingContextPlayer" 0 (struct))
      (`EnhancedInputSubsystemInterface.AddMappingContext` _returnvalue "/Game/Le_Labyrinthe/Mapping/IMC_InteractMappingContext.IMC_InteractMappingContext" 0 (struct))
      (bind _asbp_first_person_character (cast `/Game/Le_Labyrinthe/Blueprints/BP_FirstPersonCharacter` (`GameplayStatics.GetPlayerCharacter` 0)))
      (set `self.PlayerCharacter` _asbp_first_person_character)
      (set `self.TraceRange` 500.0))))

(event `EnhancedInput|/Game/Le_Labyrinthe/Mapping/IA_Move`
  (params (ActionValue :type "Vector2D Structure") (ElapsedSeconds :type "Float (double-precision)") (TriggeredSeconds :type "Float (double-precision)") (InputAction :type "InputAction Object Reference" :default "/Game/Le_Labyrinthe/Mapping/IA_Move.IA_Move"))
  (bind (_returnvalue_roll _returnvalue_pitch _returnvalue_yaw) (`KismetMathLibrary.BreakRotator` (`self.GetControlRotation`)))
  (:`Triggered`
    (`Pawn.AddMovementInput` (`self.PlayerCharacter`) (`KismetMathLibrary.GetRightVector` (`KismetMathLibrary.MakeRotator` _returnvalue_roll 0.0 _returnvalue_yaw)) ActionValue_X false)
    (`Pawn.AddMovementInput` (`self.PlayerCharacter`) (`KismetMathLibrary.GetForwardVector` (`KismetMathLibrary.MakeRotator` 0.0 0.0 _returnvalue_yaw)) ActionValue_Y false)))

(event `EnhancedInput|/Game/Le_Labyrinthe/Mapping/IA_Mouse`
  (params (ActionValue :type "Vector2D Structure") (ElapsedSeconds :type "Float (double-precision)") (TriggeredSeconds :type "Float (double-precision)") (InputAction :type "InputAction Object Reference" :default "/Game/Le_Labyrinthe/Mapping/IA_Mouse.IA_Mouse"))
  (:`Triggered`
    (`self.AddYawInput` ActionValue_X)
    (`self.AddPitchInput` ActionValue_Y)))

(event `EnhancedInput|/Game/Le_Labyrinthe/Mapping/IA_Interact`
  (params (ActionValue :type Boolean) (ElapsedSeconds :type "Float (double-precision)") (TriggeredSeconds :type "Float (double-precision)") (InputAction :type "InputAction Object Reference" :default "/Game/Le_Labyrinthe/Mapping/IA_Interact.IA_Interact"))
  (bind _returnvalue (`self.K2_GetActorLocation` (`self.PlayerCharacter`)))
  (:`Triggered`
    (bind _outhit (`KismetSystemLibrary.LineTraceSingle` :`Start` _returnvalue :`End` (+ (+ _returnvalue (0.0 0.0 75.0)) (* (`KismetMathLibrary.GetForwardVector` (`.OutRotation` (`self.GetActorEyesViewPoint`))) (`self.TraceRange`))) :`TraceChannel` "TraceTypeQuery3" :`DrawDebugType` "Persistent"))
    (bind _asbp_torche (cast `/Game/Le_Labyrinthe/Blueprints/BP_Torche` (`.HitActor` (`GameplayStatics.BreakHitResult` _outhit)))
      (:`then`
        (`/Game/Le_Labyrinthe/Blueprints/BP_Torche.ActivateFlame` _asbp_torche))
      (:`CastFailed`
        (bind _asbp_switch (cast `/Game/Le_Labyrinthe/Blueprints/BP_Switch` (`.HitActor` (`GameplayStatics.BreakHitResult` _outhit)))
          (:`then`
            (`/Game/Le_Labyrinthe/Blueprints/BP_Switch.GetInteract` _asbp_switch))
          (:`CastFailed`
            (bind _asbp_passage_secret (cast `/Game/Le_Labyrinthe/Blueprints/BP_PassageSecret` (`.HitActor` (`GameplayStatics.BreakHitResult` _outhit))))
            (`/Game/Le_Labyrinthe/Blueprints/BP_PassageSecret.Interact` _asbp_passage_secret)))))))

(fn `UserConstructionScript`)