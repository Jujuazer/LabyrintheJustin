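; BP_Torche is a torch for the labyrinth game whose flame can be toggled on and off.
; The ActivateFlame event flips IsON, activates or deactivates the PFire effect, and passes the new state to GI_GameInstance through its Torch function.
; An IsDelay flag with a half-second Delay blocks repeated toggles right after each switch.
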(event `ActivateFlame`
  (bind _p_fire (`self.P_Fire`))
  (if (not (`self.isDelay`))
    ;[1 0.5656 0.5656] Activate and set bool to game Instance
    (if (`self.isON`)
      (bind _asgi_game_instance (cast `/Game/Le_Labyrinthe/Blueprints/GI_GameInstance` (`GameplayStatics.GetGameInstance`)))
      (`/Game/Le_Labyrinthe/Blueprints/GI_GameInstance.Torch` _asgi_game_instance false)
      (`ActorComponent.Deactivate` _p_fire)
      (set `self.isON` false)
      ;[1 0.6906 0.6906] Delay mechanic
      (set `self.isDelay` true)
      (`KismetSystemLibrary.Delay` 0.5)
      (set `self.isDelay` false)
      (else
        (bind _asgi_game_instance_2 (cast `/Game/Le_Labyrinthe/Blueprints/GI_GameInstance` (`GameplayStatics.GetGameInstance`)))
        (`/Game/Le_Labyrinthe/Blueprints/GI_GameInstance.Torch` _asgi_game_instance_2 true)
        (`ActorComponent.Activate` _p_fire false)
        (set `self.isON` true)
        (set `self.isDelay` true)
        (`KismetSystemLibrary.Delay` 0.5)
        (set `self.isDelay` false)))))

(fn `UserConstructionScript`)