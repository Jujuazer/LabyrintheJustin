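; BP_Switch is an interactable lever switch that toggles between on and off.
; On interaction it flips IsOn and reattaches the Lever mesh to the Cube's On or Off socket, starting at Off on BeginPlay.
; Each toggle passes the new state to GI_GameInstance through its Switch function.
; An IsDelay flag with a short Delay blocks repeated interactions until the cooldown ends.
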(event `self.ReceiveBeginPlay`
  ;[1 0.7198 0.7198] attach cylinder to OFF socket to first socket
  (`SceneComponent.K2_AttachToComponent` (`self.lever`) (`self.cube`) "Off" "KeepRelative" "KeepRelative" "KeepRelative" true))

(event `GetInteract`
  ;[1 0.5077 0.3042] If the switch is on change socket to ON and bool to ON after 0.2s switch to off so it can be on again
  (if (`self.IsDelay`)
    _
    (elif (`self.IsOn`)
      (`SceneComponent.K2_AttachToComponent` (`self.lever`) (`self.cube`) "Off" "KeepRelative" "KeepRelative" "KeepRelative" true)
      (bind _output_get (set `self.IsOn` false))
      (bind _asgi_game_instance (cast `/Game/Le_Labyrinthe/Blueprints/GI_GameInstance` (`GameplayStatics.GetGameInstance`)))
      (`/Game/Le_Labyrinthe/Blueprints/GI_GameInstance.Switch` _asgi_game_instance _output_get)
      (set `self.IsDelay` true)
      (`KismetSystemLibrary.Delay` 0.5)
      (set `self.IsDelay` false)
      (else
        (`SceneComponent.K2_AttachToComponent` (`self.lever`) (`self.cube`) "On" "KeepRelative" "KeepRelative" "KeepRelative" true)
        (bind _output_get_2 (set `self.IsOn` true))
        (bind _asgi_game_instance_2 (cast `/Game/Le_Labyrinthe/Blueprints/GI_GameInstance` (`GameplayStatics.GetGameInstance`)))
        (`/Game/Le_Labyrinthe/Blueprints/GI_GameInstance.Switch` _asgi_game_instance_2 _output_get_2)
        (set `self.IsDelay` true)
        (`KismetSystemLibrary.Delay` 0.5)
        (set `self.IsDelay` false)))))

(fn `UserConstructionScript`
  (set `self.IsOn` false))